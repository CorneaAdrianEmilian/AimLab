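; BP_Target is a shooting target actor that scores points when a BP_Bullet overlaps it.
; On overlap it flags the bullet as a hit, then increments the player character's hit count and adds score.
; It then alternates position via an IsCentered flag, jumping to a random spot on a fixed X plane or back to a fixed center point.
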(event `self.ReceiveActorBeginOverlap`
  (params (OtherActor :type "Actor Object Reference"))
  (bind _asbp_bullet (cast `/Game/Blueprints/BP_Bullet` OtherActor))
  (set `/Game/Blueprints/BP_Bullet.Hit target` true _asbp_bullet)
  (bind _asbp_game_character (cast `/Game/Blueprints/BP_GameCharacter` (`GameplayStatics.GetPlayerCharacter` 0)))
  (`/Engine/EditorBlueprintResources/StandardMacros.IncrementInt` (`/Game/Blueprints/BP_GameCharacter.TargetsHit` _asbp_game_character)
    (:`  `
      (`/Game/Blueprints/BP_GameCharacter.Update Score` _asbp_game_character 1000)
      (if (`self.IsCentered`)
        (set `self.IsCentered` false)
        (`self.K2_SetActorLocation` (`KismetMathLibrary.MakeVector` 360.0 (`KismetMathLibrary.Conv_IntToDouble` (`KismetMathLibrary.RandomIntegerInRange` -400 400)) (`KismetMathLibrary.Conv_IntToDouble` (`KismetMathLibrary.RandomIntegerInRange` 120 340))))
        (else
          (set `self.IsCentered` true)
          (`self.K2_SetActorLocation` (360.0 10.0 210.0)))))))

(fn `UserConstructionScript`)