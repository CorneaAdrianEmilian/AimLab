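; BP_Bullet is a reusable player projectile that toggles between hidden and fired states and penalizes misses.
; Overlapping a BP_Bullet_Collision_hide_wall calls HideBullet, which hides the actor and stops ProjectileMovement ticking.
; Hiding without HitTarget set deducts score through BP_GameCharacter; a set flag is cleared instead.
; Unhiding resumes movement along the player's ArrowComponent forward vector, without repositioning the bullet.
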(event `self.ReceiveActorBeginOverlap`
  (params (OtherActor :type "Actor Object Reference"))
  (cast `/Game/Blueprints/BP_Bullet_Collision_hide_wall` OtherActor)
  (`self.Hide Bullet` true))

(fn `Hide Bullet`
  (params (Hide :type Boolean))
  (bind _projectilemovement (`self.ProjectileMovement`))
  (bind _output_get (set `self.Is hidden` Hide))
  (if _output_get
    (`ActorComponent.SetComponentTickEnabled` _projectilemovement false)
    (`self.SetActorHiddenInGame` true)
    (if (`self.Hit target`)
      (set `self.Hit target` false)
      (else
        (bind _asbp_game_character (cast `/Game/Blueprints/BP_GameCharacter` (`GameplayStatics.GetPlayerCharacter` 0)))
        (`/Game/Blueprints/BP_GameCharacter.Update Score` _asbp_game_character -500)
        (set `self.Hit target` false)))
    (else
      (`ActorComponent.SetComponentTickEnabled` _projectilemovement true)
      (`self.SetActorHiddenInGame` false)
      (set `MovementComponent.Velocity` (* (`SceneComponent.GetForwardVector` (`self.GetComponentByClass` (`GameplayStatics.GetPlayerCharacter` 0) "/Script/Engine.ArrowComponent")) 5000.0) _projectilemovement))))

(fn `UserConstructionScript`)